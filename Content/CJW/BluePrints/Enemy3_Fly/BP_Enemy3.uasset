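; Flying enemy that patrols, winds up and charges the player, damaging and destroying itself on any actor overlap.
; Tick runs an externally set Mode: patrol along normalized PatrolLocation, hold with effects and sound, or home in.
; PatrolLocation periodically takes the player's world position and is overwritten at height limits.
; Damage knocks it away from the player, low HP sets glory-mode flags, and death spawns armor, bullet and HP pickups.
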(event EventBeginPlay
  (bind _returnvalue (Math|Random|RandomFloatinRange 3e+02 -3e+02))
  (Variables|Default|SetPatrolLocation (Math|Vector|MakeVector _returnvalue _returnvalue _returnvalue)))

(event Collision|EventActorBeginOverlap
  (params (OtherActor :type Actor%20Object%20Reference))
  (Game|Damage|ApplyDamage OtherActor (Variables|Default|Getdamage) 0 0)
  (Actor|DestroyActor)
  (Effects|SpawnEmitteratLocation "/Game/Realistic_Starter_VFX_Pack_Vol2/Particles/Blood/P_Blood_Splat_Cone.P_Blood_Splat_Cone" (Transformation|GetActorLocation) "0, 0, 0" "3.000000,3.000000,3.000000"))

(event EventTick
  (params (DeltaSeconds :type Float%20%28single-precision%29))
  (Utilities|FlowControl|Sequence
    (:then_0
      (if (<= (Variables|Default|GetHP) 40)
        (Variables|Default|SetIsGloryMode_0 true)))
    (:then_1
      (Utilities|FlowControl|Sequence
        (:then_0
          (Utilities|FlowControl|Delay 3.0)
          (Variables|Default|SetPatrolLocation (Transformation|GetActorLocation (Game|Player|GetPlayerPawn 0))))
        (:then_1
          (switch int (Variables|Default|GetMode)
            (:0
              ;[1 1 1] 순찰모드
              (CallFunction|GotoTarget(Patrol)))
            (:1
              (CallFunction|Wait))
            (:2
              (CallFunction|GotoTarget(Player)))))
        (:then_2
          (Variables|Default|SetCurrentLocation (Transformation|GetActorTransform)))
        (:then_3
          ;[1 1 1] 높이 날기 제한
          (Utilities|FlowControl|Sequence
            (:then_0
              (if (>= (.z (Transformation|GetActorLocation)) 1.5e+03)
                (Variables|Default|SetPatrolLocation (Math|Vector|MakeVector 0.0 0.0 (- (.z (Variables|Default|GetPatrolLocation)) 1.0)))))
            (:then_1
              (if (< (.z (Transformation|GetActorLocation)) 6e+01)
                (Variables|Default|SetPatrolLocation (Math|Vector|MakeVector 0.0 0.0 (+ (.z (Variables|Default|GetPatrolLocation)) 1.0)))))))))))

(event Game|Damage|EventAnyDamage
  (params (Damage :type Float%20%28single-precision%29) (DamageType :type Damage%20Type%20Object%20Reference) (InstigatedBy :type Controller%20Object%20Reference) (DamageCauser :type Actor%20Object%20Reference))
  (bind _returnvalue (Transformation|GetActorLocation))
  (bind _output_get (Variables|Default|SetHP (Math|Float|Truncate (- (Variables|Default|GetHP) Damage))))
  (Utilities|FlowControl|Sequence
    (:then_0
      (Transformation|SetActorLocation (+ (Transformation|GetActorLocation) (* (Math|Vector|Normalize (- (Transformation|GetActorLocation (Game|Player|GetPlayerPawn 0)) (Transformation|GetActorLocation))) "-15.000000,-15.000000,-15.000000")) false true))
    (:then_1
      (if (<= _output_get 0)
        (Effects|SpawnEmitteratLocation "/Game/Realistic_Starter_VFX_Pack_Vol2/Particles/Blood/P_Blood_Splat_Cone.P_Blood_Splat_Cone" (Transformation|GetActorLocation self) "0, 0, 0" "4.000000,4.000000,4.000000")
        (Utilities|FlowControl|Delay 0.5)
        (Actor|DestroyActor)
        (Utilities|FlowControl|Sequence
          (:then_0
            (Game|SpawnActorfromClass "/Game/CJW/BluePrints/BulletItem/Armor/BP_Armor.BP_Armor_C" (Math|Conversions|ToTransform(Vector) _returnvalue) "Undefined" "MultiplyWithRoot" 0 0))
          (:then_1
            (Game|SpawnActorfromClass "/Game/CJW/BluePrints/BulletItem/Bullet/BP_Bullet.BP_Bullet_C" (Math|Conversions|ToTransform(Vector) _returnvalue) "Undefined" "MultiplyWithRoot" 0 0))
          (:then_2
            (Game|SpawnActorfromClass "/Game/CJW/BluePrints/BulletItem/HP/BP_HP.BP_HP_C" (Math|Conversions|ToTransform(Vector) _returnvalue) "Undefined" "MultiplyWithRoot" 0 0)))
        (else
          (Utilities|FlowControl|Sequence
            (:then_0
              (if (<= (Variables|Default|GetHP) 50)
                (Variables|Default|SetIsGloryMode true)))
            (:then_1
              (Utilities|IsValid "/Game/CJW/Widget/WB_HitMotion.WB_HitMotion"))))))))

(fn ConstructionScript)

(fn SetPatrolMode
  (Variables|Default|SetMode 0))

(fn GotoTarget(Patrol)
  (Transformation|SetActorLocation (+ (Transformation|GetActorLocation) (* (Variables|Default|GetPatrolSpeed) (Utilities|Time|GetWorldDeltaSeconds) (Math|Vector|Normalize (Variables|Default|GetPatrolLocation)))) false false)
  (Variables|Default|SetNewVar false))

(fn SetWaitMode
  (Variables|Default|SetMode 1))

(fn SetAttackMode
  (Variables|Default|SetMode 2))

(fn Wait
  (bind _returnvalue (Transformation|GetActorLocation))
  (Transformation|SetActorLocation (.location (Variables|Default|GetCurrentLocation)) false false)
  (Transformation|SetActorRotation (Math|Rotator|FindLookatRotation (Transformation|GetActorLocation (Game|Player|GetPlayerPawn 0)) _returnvalue))
  (Transformation|AddActorLocalRotation "0.000000,90.000000,0.000000" false false)
  (Effects|SpawnEmitteratLocation "/Game/Realistic_Starter_VFX_Pack_Vol2/Particles/Hit/P_Brick.P_Brick" _returnvalue "0, 0, 0" "0.800000,0.800000,0.800000")
  (if (not (Variables|Default|GetNewVar))
    (Audio|PlaySound2D "/Game/CJW/Sounds/Enemy2Attackmode.Enemy2Attackmode" 1.0 1.0 0.0 0 0)
    (Variables|Default|SetNewVar true)))

(fn GotoTarget(Player)
  (Transformation|SetActorLocation (+ (Transformation|GetActorLocation) (* (Variables|Default|GetAttackSpeed) (Utilities|Time|GetWorldDeltaSeconds) (Math|Vector|Normalize (- (Transformation|GetActorLocation (Game|Player|GetPlayerPawn 0)) (Transformation|GetActorLocation))) "1.000000,1.000000,1.000000")) false false)
  (Transformation|SetActorRotation (Math|Rotator|FindLookatRotation (Transformation|GetActorLocation (Game|Player|GetPlayerPawn 0)) (Transformation|GetActorLocation)))
  (Transformation|AddActorLocalRotation "0.000000,90.000000,0.000000" false false))

(fn NewFunction)