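; BP_MiddleBossAi is the AI controller for the middle boss, starting the BT_MiddleBoss behavior tree on BeginPlay.
; AI Perception updates pass each actor to GetPlayerActor, which acts only on actors tagged "Player".
; It toggles the MiddleBossActorKey blackboard object, clearing it if already valid and otherwise storing the player, without checking whether the stimulus was gained or lost.
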(event OnPerceptionUpdated(AIPerception)
  (params (UpdatedActors :type Array%20of%20Actor%20Object%20References))
  (for _array_element UpdatedActors
    (CallFunction|GetPlayerActor _array_element)))

(event EventBeginPlay
  (AI|RunBehaviorTree "/Game/CJW/BluePrints/Middle_Boss/BT_MiddleBoss.BT_MiddleBoss"))

(event EventTick
  (params (DeltaSeconds :type Float%20%28single-precision%29)))

(fn ConstructionScript)

(fn GetPlayerActor
  (params (SensedActor :type Actor%20Object%20Reference))
  (if (Actor|ActorHasTag SensedActor "Player")
    (Utilities|IsValid (AI|Components|Blackboard|GetValueasObject (AI|GetBlackboard 0) (Utilities|Name|MakeLiteralName "MiddleBossActorKey"))
      (:Is%20Valid
        (AI|Components|Blackboard|SetValueasObject (AI|GetBlackboard 0) (Utilities|Name|MakeLiteralName "MiddleBossActorKey") 0))
      (:Is%20Not%20Valid
        (AI|Components|Blackboard|SetValueasObject (AI|GetBlackboard 0) (Utilities|Name|MakeLiteralName "MiddleBossActorKey") SensedActor)))))