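; Middle boss that hunts the player, deals damage on overlap and flashes a hit-marker widget when hurt.
; Tick faces the player and moves by Mode (dash, frame-counted charge at the last stored player position, slow follow) using unswept location offsets.
; Setter functions switch modes, while Tick exchanges distance and timer values with the Blackboard.
; Death spawns blood, updates BP_ThroneRoom's level and shows the game-clear screen.
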(event Collision|EventActorBeginOverlap
  (params (OtherActor :type Actor%20Object%20Reference))
  ;[1 1 1] 플레이어한테 데미지 입히기
  (Game|Damage|ApplyDamage OtherActor (Variables|Default|Getdamage) 0 0))

(event EventTick
  (params (DeltaSeconds :type Float%20%28single-precision%29))
  (bind _returnvalue (Game|Player|GetPlayerPawn 0))
  (Utilities|IsValid _returnvalue
    (:Is%20Valid
      (Utilities|FlowControl|Sequence
        (:then_0
          ;[1 1 1] 가는방향을 바라보도록 하기
          (Transformation|SetActorRotation (Math|Rotator|FindLookatRotation (Transformation|GetActorLocation) (Transformation|GetActorLocation (Game|Player|GetPlayerPawn 0)))))
        (:then_1
          (switch int (Variables|Default|GetMode)
            (:1
              ;[1 1 1] 전방 대쉬
              (if (<= (Class|BlackboardComponent|GetValueasFloat (AI|GetBlackboard 0) (Utilities|Name|MakeLiteralName "MiddleBossDistanceToPlayer")) 4e+02)
                (Variables|Default|SetMode 0)
                (else
                  (CallFunction|Goto 5e+04 (.location (Transformation|GetActorTransform (Game|Player|GetPlayerPawn 0)))))))
            (:2
              (if (>= (Variables|Default|GetAttackTime) 6e+01)
                ;[1 1 1] Comment
                ;;[1 1 1] 전방 도끼스윙하고 다시 초기화
                (AI|Components|Blackboard|SetValueasFloat (AI|GetBlackboard 0) (Utilities|Name|MakeLiteralName "MiddleBossWaitTimeKey") 0.0)
                (Variables|Default|SetAttackTime 0.0)
                (else
                  ;[1 1 1] 쿨이 20보다 작다면 1500의 속도로
                  (CallFunction|Goto 2.5e+03 (Variables|Default|GetPlayerLocation))
                  (Math|Float|IncrementFloat (Variables|Default|GetAttackTime)))))
            (:3
              (Utilities|FlowControl|Sequence
                (:then_1
                  (Variables|Default|SetPlayerLocation (Transformation|GetActorLocation _returnvalue))
                  (CallFunction|Goto 3e+02 (Variables|Default|GetPlayerLocation)))))
            (:4
              (CallFunction|Goto 2e+04 (Math|Vector|MakeVector 1e+03 1e+03 0.0)))))
        (:then_2
          (Utilities|IsValid "BP_MiddleBoss"
            (:Is%20Valid
              ;[1 1 1] 타임사이클 최신화
              (Variables|Default|SetCurrentTimeCycle (Class|BlackboardComponent|GetValueasFloat (AI|GetBlackboard 0) (Utilities|Name|MakeLiteralName "MiddleBossTimeCycle"))))))))))

(event EventBeginPlay
  (Variables|Default|SetHP (Variables|Default|GetMaxHp)))

(event Game|Damage|EventAnyDamage
  (params (Damage :type Float%20%28single-precision%29) (DamageType :type Damage%20Type%20Object%20Reference) (InstigatedBy :type Controller%20Object%20Reference) (DamageCauser :type Actor%20Object%20Reference))
  (bind _output_get (Variables|Default|SetHP (- (Variables|Default|GetHP) Damage)))
  (if (<= _output_get 0)
    ;[1 1 1] Comment
    (Actor|DestroyActor)
    (Effects|SpawnEmitteratLocation "/Game/Realistic_Starter_VFX_Pack_Vol2/Particles/Blood/P_Blood_Splat_Cone.P_Blood_Splat_Cone" "0, 0, 0")
    (bind _returnvalue (Actor|GetActorOfClass "/Game/EnvironmentPack1/Blueprints/BP_ThroneRoom.BP_ThroneRoom_C"))
    (bind _asbp_throne_room (Utilities|Casting|CastToBP_ThroneRoom _returnvalue))
    (Variables|/Game/EnvironmentPack1/Blueprints/BP_ThroneRoom.BP_ThroneRoom_C|SetCurrentLevel _asbp_throne_room 1.0)
    (bind _returnvalue_2 (UserInterface|CreateWidget "/Game/CJW/WBP_Gameclear.WBP_Gameclear_C"))
    (UserInterface|Viewport|AddtoViewport _returnvalue_2 0)
    (UserInterface|Animation|PlayAnimation _returnvalue_2 (Variables|/Game/CJW/WBP_Gameclear.WBP_Gameclear_C|GetNewAnimation _returnvalue_2) 0.0 1 "Forward" 1.0 false)
    (else
      (Utilities|IsValid "/Game/CJW/Widget/WB_HitMotion.WB_HitMotion"
        (:Is%20Valid
          (Utilities|IsValid (Variables|Default|GetCrosshair)
            (:Is%20Valid
              _)
            (:Is%20Not%20Valid
              (bind _returnvalue_3 (UserInterface|CreateWidget "/Game/CJW/Widget/WB_HitMotion.WB_HitMotion_C"))
              (Variables|Default|SetCrosshair _returnvalue_3)))
          (UserInterface|Viewport|AddtoViewport (Variables|Default|GetCrosshair) 0)
          (Utilities|FlowControl|Delay 0.2)
          (Widget|RemovefromParent (Variables|Default|GetCrosshair)))))))

(fn ConstructionScript)

(fn Goto
  (params (Speed :type Float%20%28double-precision%29) (targetactor :type Vector))
  (Transformation|SetActorLocation (+ (Transformation|GetActorLocation) (* Speed (Utilities|Time|GetWorldDeltaSeconds) (Math|Vector|Normalize (- targetactor (Transformation|GetActorLocation))))) false false))

(fn SetAttackMode
  (Variables|Default|SetMode 2))

(fn SetDashMode
  (Variables|Default|SetMode 1))

(fn SetWaitMode
  (Variables|Default|SetMode 3))