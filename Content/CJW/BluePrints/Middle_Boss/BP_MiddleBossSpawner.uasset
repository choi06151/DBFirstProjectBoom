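; BP_MiddleBossSpawner is a one-shot trigger actor that spawns the middle boss when the player character overlaps it.
; On overlap with BP_FirstPersonCharacter, it spawns BP_MiddleBoss at a hardcoded position, destroys itself and emits a stretched ambient dust effect at its own location.
; An unconnected branch that would spawn the boss at the spawner's location based on the game mode's CurrenTime never runs.
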(event EventBeginPlay)

(event Collision|EventActorBeginOverlap
  (params (OtherActor :type Actor%20Object%20Reference))
  (Utilities|Casting|CastToBP_FirstPersonCharacter OtherActor)
  (Game|SpawnActorfromClass "/Game/CJW/BluePrints/Middle_Boss/BP_MiddleBoss.BP_MiddleBoss_C" (Math|Transform|MakeTransform "-90.000000,-60.000000,150.000000" "0, 0, 0" "1.000000,1.000000,1.000000") "Undefined" "MultiplyWithRoot" 0 0)
  (Actor|DestroyActor)
  (Effects|SpawnEmitteratLocation "/Game/JIU/StarterContent/Particles/P_Ambient_Dust.P_Ambient_Dust" (Transformation|GetActorLocation) "0, 0, 0" "5.000000,1.000000,1.000000"))

(fn ConstructionScript)