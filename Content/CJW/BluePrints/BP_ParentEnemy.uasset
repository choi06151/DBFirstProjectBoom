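; BP_ParentEnemy is a parent enemy Blueprint that handles taking damage and dying.
; AnyDamage lowers HP and teleports the enemy slightly away from the player as knockback.
; Surviving hits briefly show a WB_HitMotion crosshair widget, and low HP sets IsGloryMode.
; Death spawns blood, then after a delay destroys the actor, increments KilledEnemyTimes, plays a sound and drops armor, bullet and HP pickups.
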(event EventBeginPlay)

(event Collision|EventActorBeginOverlap
  (params (OtherActor :type Actor%20Object%20Reference)))

(event EventTick
  (params (DeltaSeconds :type Float%20%28single-precision%29)))

(event Game|Damage|EventAnyDamage
  (params (Damage :type Float%20%28single-precision%29) (DamageType :type Damage%20Type%20Object%20Reference) (InstigatedBy :type Controller%20Object%20Reference) (DamageCauser :type Actor%20Object%20Reference))
  (bind _returnvalue (Transformation|GetActorLocation))
  (bind _output_get (Variables|Default|SetHP (Math|Float|Truncate (- (Variables|Default|GetHP) Damage))))
  (Utilities|FlowControl|Sequence
    (:then_0
      (Transformation|SetActorLocation (+ (Transformation|GetActorLocation) (* (Math|Vector|Normalize (- (Transformation|GetActorLocation (Game|Player|GetPlayerPawn 0)) (Transformation|GetActorLocation))) "-15.000000,-15.000000,-15.000000")) false true))
    (:then_1
      (if (<= _output_get 0)
        (Effects|SpawnEmitteratLocation "/Game/Realistic_Starter_VFX_Pack_Vol2/Particles/Blood/P_Blood_Splat_Cone.P_Blood_Splat_Cone" (Transformation|GetActorLocation self) "0, 0, 0" "4.000000,4.000000,4.000000")
        (Utilities|FlowControl|Delay 0.5)
        (Actor|DestroyActor)
        (Variables|Default|SetKilledEnemyTimes (+ (Variables|Default|GetKilledEnemyTimes) 1))
        (Utilities|FlowControl|Sequence
          (:then_0
            (Game|SpawnActorfromClass "/Game/CJW/BluePrints/BulletItem/Armor/BP_Armor.BP_Armor_C" (Math|Conversions|ToTransform(Vector) _returnvalue) "Undefined" "MultiplyWithRoot" 0 0)
            (Audio|PlaySoundatLocation "/Game/CJW/Sounds/diezombie.diezombie" (Transformation|GetActorLocation) "0, 0, 0" 1.0 1.0 0.0 0 0 0 0))
          (:then_1
            (Game|SpawnActorfromClass "/Game/CJW/BluePrints/BulletItem/Bullet/BP_Bullet.BP_Bullet_C" (Math|Conversions|ToTransform(Vector) _returnvalue) "Undefined" "MultiplyWithRoot" 0 0))
          (:then_2
            (Game|SpawnActorfromClass "/Game/CJW/BluePrints/BulletItem/HP/BP_HP.BP_HP_C" (Math|Conversions|ToTransform(Vector) _returnvalue) "Undefined" "MultiplyWithRoot" 0 0)))
        (else
          (Utilities|FlowControl|Sequence
            (:then_0
              (if (<= (Variables|Default|GetHP) 50)
                (Variables|Default|SetIsGloryMode true)))
            (:then_1
              (Utilities|IsValid "/Game/CJW/Widget/WB_HitMotion.WB_HitMotion"
                (:Is%20Valid
                  (Utilities|IsValid (Variables|Default|GetCrosshair)
                    (:Is%20Valid
                      _)
                    (:Is%20Not%20Valid
                      (bind _returnvalue_2 (UserInterface|CreateWidget "/Game/CJW/Widget/WB_HitMotion.WB_HitMotion_C"))
                      (Variables|Default|SetCrosshair _returnvalue_2)))
                  (UserInterface|Viewport|AddtoViewport (Variables|Default|GetCrosshair) 0)
                  (Utilities|FlowControl|Delay 0.2)
                  (Widget|RemovefromParent (Variables|Default|GetCrosshair)))))))))))

(fn ConstructionScript)