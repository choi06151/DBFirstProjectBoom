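; BP_Enemy4 is a tentacle enemy that applies damage to any actor it overlaps.
; Its Mode, set by wait, patrol, attack and come-back functions, decides whether Tick moves it straight toward a Blackboard target location, back toward a return location, or neither.
; At low HP, Tick hides the Tentacle component, shows the Glorymode one and sets a glory-mode flag.
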(event EventBeginPlay)

(event Collision|EventActorBeginOverlap
  (params (OtherActor :type Actor%20Object%20Reference))
  (Game|Damage|ApplyDamage OtherActor (Variables|Default|Getdamage) 0 0))

(event EventTick
  (params (DeltaSeconds :type Float%20%28single-precision%29))
  (Utilities|FlowControl|Sequence
    (:then_0
      (if (<= (Variables|Default|GetHP_0) 40)
        (Rendering|SetVisibility (Variables|Default|Gettentacle) false false)
        (Rendering|SetVisibility (Variables|Default|GetGlorymode) true false)
        (Variables|Default|SetIsGloryMode_0 true)))
    (:then_1
      (switch int (Variables|Default|GetMode)
        (:1
          (CallFunction|GotoTarget(Target)))
        (:2
          (CallFunction|Returnback))))))

(fn ConstructionScript)

(fn SetWaitMode
  (Variables|Default|SetMode 0))

(fn SetAttackMode
  (Variables|Default|SetMode 1))

(fn GotoTarget(Target)
  (Transformation|SetActorLocation (+ (Transformation|GetActorLocation) (* (Variables|Default|GetAttackSpeed) (Utilities|Time|GetWorldDeltaSeconds) (Math|Vector|Normalize (- (AI|Components|Blackboard|GetValueasVector (AI|GetBlackboard 0) (Utilities|Name|MakeLiteralName "Enemy4TargetKey")) (Transformation|GetActorLocation))))) false false))

(fn Returnback
  (Transformation|SetActorLocation (+ (Transformation|GetActorLocation) (* (Variables|Default|GetAttackSpeed) (Utilities|Time|GetWorldDeltaSeconds) (Math|Vector|Normalize (- (AI|Components|Blackboard|GetValueasVector (AI|GetBlackboard 0) (Utilities|Name|MakeLiteralName "Enemy4ComeBackKey")) (Transformation|GetActorLocation))))) false false))

(fn SetPatrolMode
  (Variables|Default|SetMode 0))

(fn SetComeBackMode
  (Variables|Default|SetMode 2))