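; BP_Armor is an armor pickup that homes in on the player and adds to the first-person character's Armor.
; Any actor overlap sets ComePlayer, after which Tick moves it toward the player pawn at a scaled Speed while incrementing its roll.
; A per-tick distance check destroys it at very close range and grants the armor.
; Its Cube component is hidden shortly after BeginPlay.
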(event EventBeginPlay
  (Utilities|FlowControl|Delay 2.0)
  (Rendering|SetVisibility (Variables|Default|GetCube) false false))

(event Collision|EventActorBeginOverlap
  (params (OtherActor :type Actor%20Object%20Reference))
  (Variables|Default|SetComePlayer true))

(event EventTick
  (params (DeltaSeconds :type Float%20%28single-precision%29))
  (Utilities|FlowControl|Sequence
    (:then_0
      (if (<= (Math|Vector|Distance(Vector) (Transformation|GetActorLocation) (Transformation|GetActorLocation (Game|Player|GetPlayerPawn 0))) 1e+01)
        (Actor|DestroyActor)
        (bind _asbp_first_person_character (Utilities|Casting|CastToBP_FirstPersonCharacter (Game|Player|GetPlayerPawn 0)))
        (Variables|/Game/JIU/FirstPerson/Blueprints/BP_FirstPersonCharacter.BP_FirstPersonCharacter_C|SetArmor _asbp_first_person_character (Math|Conversions|ToFloat(Integer) (+ (Variables|/Game/JIU/FirstPerson/Blueprints/BP_FirstPersonCharacter.BP_FirstPersonCharacter_C|GetArmor _asbp_first_person_character) 10)))))
    (:then_1
      (if (Variables|Default|GetComePlayer)
        (Transformation|SetActorLocation (+ (Transformation|GetActorLocation) (* (Variables|Default|GetSpeed) (Utilities|Time|GetWorldDeltaSeconds) (Math|Vector|Normalize (- (Transformation|GetActorLocation (Game|Player|GetPlayerPawn 0)) (Transformation|GetActorLocation))) (Math|Trig|Sin(Radians) 2.0))) false false)
        (bind _result (Math|Float|IncrementFloat (Variables|Default|Getrotate))
          (:%20%20
            (Transformation|SetActorRotation (Math|Rotator|MakeRotator _result 0.0 0.0))))))))

(fn ConstructionScript)