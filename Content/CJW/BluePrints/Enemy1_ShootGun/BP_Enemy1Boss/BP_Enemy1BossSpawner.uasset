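; Spawner actor that places BP_Enemy1Boss enemies at its own location, starting with one on BeginPlay.
; While State is 0, a Delay on Tick paces further spawns, counted by Spawntimes.
; On reaching the spawn limit it destroys itself and marks BP_ThroneRoom stage clear, without checking boss deaths.
; State 1 destroys the spawner immediately, and a game mode Stage switch is left unconnected.
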(event EventBeginPlay
  (Game|SpawnActorfromClass "/Game/CJW/BluePrints/Enemy1_ShootGun/BP_Enemy1Boss/BP_Enemy1Boss.BP_Enemy1Boss_C" (Math|Conversions|ToTransform(Vector) (Transformation|GetActorLocation)) "AdjustIfPossibleButAlwaysSpawn" "MultiplyWithRoot" 0 0))

(event Collision|EventActorBeginOverlap
  (params (OtherActor :type Actor%20Object%20Reference)))

(event EventTick
  (params (DeltaSeconds :type Float%20%28single-precision%29))
  (switch int (Variables|Default|GetState)
    (:0
      (Utilities|FlowControl|Delay 1e+01)
      (Game|SpawnActorfromClass "/Game/CJW/BluePrints/Enemy1_ShootGun/BP_Enemy1Boss/BP_Enemy1Boss.BP_Enemy1Boss_C" (Math|Conversions|ToTransform(Vector) (Transformation|GetActorLocation)) "AdjustIfPossibleButAlwaysSpawn" "MultiplyWithRoot" 0 0)
      (if (>= (Variables|Default|GetSpawntimes) 2)
        (Actor|DestroyActor)
        (bind _returnvalue (Actor|GetActorOfClass "/Game/EnvironmentPack1/Blueprints/BP_ThroneRoom.BP_ThroneRoom_C"))
        (bind _asbp_throne_room (Utilities|Casting|CastToBP_ThroneRoom _returnvalue))
        (Variables|/Game/EnvironmentPack1/Blueprints/BP_ThroneRoom.BP_ThroneRoom_C|SetIsStageClear _asbp_throne_room true)
        (else
          (Variables|Default|SetSpawntimes (+ (Variables|Default|GetSpawntimes) 1)))))
    (:1
      (Actor|DestroyActor))))

(fn ConstructionScript)