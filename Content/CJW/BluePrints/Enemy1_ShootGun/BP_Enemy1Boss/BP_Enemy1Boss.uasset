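; Enemy boss actor that turns to track the player, damages overlapping actors and shows its Glorymode component once HP drops to 40 or below.
; Tick also records 2D player distance and, in mode 2, spawns BP_FireBall on a frame-counted cooldown.
; SetAttackMode sets the mode; each mode 3 call steps the boss toward the player and primes the cooldown.
; Death, item-drop and direct player HP-reduction logic is unwired.
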(event Collision|EventActorBeginOverlap
  (params (OtherActor :type Actor%20Object%20Reference))
  (Game|Damage|ApplyDamage OtherActor (Variables|Default|Getdamage) 0 0))

(event EventTick
  (params (DeltaSeconds :type Float%20%28single-precision%29))
  (Utilities|FlowControl|Sequence
    (:then_0
      (if (<= (Variables|Default|GetHP_0) 40)
        (Rendering|SetVisibility (Variables|Default|GetGlorymode) true false)
        (Variables|Default|SetIsGloryMode_0 true)))
    (:then_1
      (switch int (Variables|Default|Getmode)
        (:2
          (if (>= (Variables|Default|GetFireBallCoolTime) 1.4e+02)
            (CallFunction|Fireball)
            (Variables|Default|SetFireBallCoolTime 0.0)
            (else
              (Variables|Default|SetFireBallCoolTime (+ (Variables|Default|GetFireBallCoolTime) 1.0)))))))
    (:then_2
      (Transformation|SetActorRotation (Math|Rotator|FindLookatRotation (Transformation|GetActorLocation (Game|Player|GetPlayerPawn 0)) (Transformation|GetActorLocation)))
      (Transformation|AddActorLocalRotation "0.000000,90.000000,0.000000" false false))
    (:then_3
      (Variables|Default|Setfirevallmode (Math|Vector|Distance2D(Vector) (Math|Conversions|ToVector2D(Vector) (Transformation|GetActorLocation (Game|Player|GetPlayerPawn 0))) (Math|Conversions|ToVector2D(Vector) (Transformation|GetActorLocation)))))))

(fn ConstructionScript)

(fn SetAttackMode
  (params (mode :type Integer))
  (bind _output_get (Variables|Default|Setmode mode))
  (switch int _output_get
    (:3
      (Transformation|SetActorLocation (+ (Transformation|GetActorLocation) (* (Variables|Default|GetSpeed) (Utilities|Time|GetWorldDeltaSeconds) (Math|Vector|Normalize (- (Transformation|GetActorLocation (Game|Player|GetPlayerPawn 0)) (Transformation|GetActorLocation))))) false false)
      (Variables|Default|SetFireBallCoolTime 1.3e+02))))

(fn Fireball
  (Game|SpawnActorfromClass "/Game/CJW/BluePrints/Enemy1_ShootGun/BP_ENemy1/BP_FireBall.BP_FireBall_C" (Math|Conversions|ToTransform(Vector) (Transformation|GetActorLocation)) "Undefined" "MultiplyWithRoot" 0 0))