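; AI controller for the Enemy1 boss that runs the BT_Enemy1Boss behavior tree on BeginPlay.
; Each perception update toggles the blackboard's ActorKey for actors tagged Player, clearing it if already valid or storing the sensed actor otherwise.
; InitPatrolMode, not called within this Blueprint, copies the controlled BP_Enemy1's two patrol point locations into the blackboard.
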(event OnPerceptionUpdated(AIPerception)
  (params (UpdatedActors :type Array%20of%20Actor%20Object%20References))
  (for _array_element UpdatedActors
    (CallFunction|CheckPlayerActor _array_element)))

(event EventBeginPlay
  (AI|RunBehaviorTree "/Game/CJW/BluePrints/Enemy1_ShootGun/BP_Enemy1Boss/BT_Enemy1Boss.BT_Enemy1Boss"))

(event EventTick
  (params (DeltaSeconds :type Float%20%28single-precision%29)))

(fn ConstructionScript)

(fn CheckPlayerActor
  (params (SensedActor :type Actor%20Object%20Reference))
  (if (Actor|ActorHasTag SensedActor "Player")
    (Utilities|IsValid (AI|Components|Blackboard|GetValueasObject (AI|GetBlackboard 0) (Utilities|Name|MakeLiteralName "ActorKey"))
      (:Is%20Valid
        (AI|Components|Blackboard|SetValueasObject (AI|GetBlackboard 0) (Utilities|Name|MakeLiteralName "ActorKey") 0))
      (:Is%20Not%20Valid
        (AI|Components|Blackboard|SetValueasObject (AI|GetBlackboard 0) (Utilities|Name|MakeLiteralName "ActorKey") SensedActor)))))

(fn InitPatrolMode
  (bind _asbp_enemy_1 (Utilities|Casting|CastToBP_Enemy1 (Pawn|GetControlledPawn)))
  (AI|Components|Blackboard|SetValueasVector (AI|GetBlackboard 0) (Utilities|Name|MakeLiteralName "PatrolPoint1") (Transformation|GetActorLocation (Variables|/Game/CJW/BluePrints/Enemy1_ShootGun/BP_ENemy1/BP_Enemy1.BP_Enemy1_C|GetPatrolPoint1 _asbp_enemy_1)))
  (AI|Components|Blackboard|SetValueasVector (AI|GetBlackboard 0) (Utilities|Name|MakeLiteralName "PatrolPoint2") (Transformation|GetActorLocation (Variables|/Game/CJW/BluePrints/Enemy1_ShootGun/BP_ENemy1/BP_Enemy1.BP_Enemy1_C|GetPatrolPoint2 _asbp_enemy_1))))