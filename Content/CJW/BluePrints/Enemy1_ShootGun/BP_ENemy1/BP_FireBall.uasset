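; BP_FireBall is a fireball projectile that flies toward the player and damages whatever it overlaps.
; On BeginPlay it locks a normalized direction to the player pawn's position, then Tick moves it along that straight line without homing or sweep.
; Tick also attaches a new fire emitter to the box every frame.
; On overlap it applies damage, destroys itself and spawns an explosion effect.
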(event EventBeginPlay
  (CallFunction|GetPlayerLocation))

(event Collision|EventActorBeginOverlap
  (params (OtherActor :type Actor%20Object%20Reference))
  (Game|Damage|ApplyDamage OtherActor (Variables|Default|Getdamage) 0 0)
  (Actor|DestroyActor)
  (Effects|SpawnEmitteratLocation "/Game/JIU/StarterContent/Particles/P_Explosion.P_Explosion" (Transformation|GetActorLocation)))

(event EventTick
  (params (DeltaSeconds :type Float%20%28single-precision%29))
  (Utilities|FlowControl|Sequence
    (:then_0
      (Transformation|SetActorLocation (+ (Transformation|GetActorLocation) (* (Utilities|Time|GetWorldDeltaSeconds) (Variables|Default|GetSpeed) (Variables|Default|GetDirection))) false false))
    (:then_1
      (Effects|SpawnEmitterAttached "/Game/JIU/StarterContent/Particles/P_Fire.P_Fire" (Variables|Default|GetBox) "None" "0, 0, 0" "0, 0, 0" "0.500000,0.500000,0.500000"))))

(fn ConstructionScript)

(fn GetPlayerLocation
  (Variables|Default|SetDirection (Math|Vector|Normalize (- (Transformation|GetActorLocation (Game|Player|GetPlayerPawn 0)) (Transformation|GetActorLocation)))))