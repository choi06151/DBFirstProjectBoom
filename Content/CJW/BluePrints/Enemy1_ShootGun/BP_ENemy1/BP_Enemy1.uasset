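; BP_Enemy1 is an enemy that damages actors it overlaps and shoots fireballs when in attack mode 2.
; Tick checks Mode and, in that mode, uses a Delay to pace Fireball to roughly once a second, spawning BP_FireBall at the enemy's location.
; SetAttackMode stores Mode, but its switch has nothing wired.
; An unconnected chain that subtracts HP from BP_FirstPersonCharacter never runs.
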(event EventBeginPlay)

(event Collision|EventActorBeginOverlap
  (params (OtherActor :type Actor%20Object%20Reference))
  (Game|Damage|ApplyDamage OtherActor (Variables|Default|Getdamage) 0 0))

(event EventTick
  (params (DeltaSeconds :type Float%20%28single-precision%29))
  (switch int (Variables|Default|Getmode)
    (:2
      (Utilities|FlowControl|Delay 1.0)
      (CallFunction|Fireball))))

(event Collision|EventHit
  (params (MyComp :type Primitive%20Component%20Object%20Reference) (Other :type Actor%20Object%20Reference) (OtherComp :type Primitive%20Component%20Object%20Reference) (bSelfMoved :type Boolean) (HitLocation :type Vector :default "0, 0, 0") (HitNormal :type Vector :default "0, 0, 0") (NormalImpulse :type Vector :default "0, 0, 0") (Hit :type Hit%20Result%20Structure%20%28by%20ref%29)))

(fn ConstructionScript)

(fn SetAttackMode
  (params (mode :type Integer))
  (bind _output_get (Variables|Default|Setmode mode))
  (switch int _output_get))

(fn Fireball
  (Game|SpawnActorfromClass "/Game/CJW/BluePrints/Enemy1_ShootGun/BP_ENemy1/BP_FireBall.BP_FireBall_C" (Math|Conversions|ToTransform(Vector) (Transformation|GetActorLocation)) "Undefined" "MultiplyWithRoot" 0 0))