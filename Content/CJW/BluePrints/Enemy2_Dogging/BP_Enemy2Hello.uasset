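; BP_Enemy2Hello is a dog enemy that homes in on the player, damaging any actor it overlaps and destroying itself.
; Tick moves it straight toward player pawn 0 and orients it with a look-at plus fixed rotation offset.
; Damage lowers HP and knocks it back, setting IsGloryMode at low health.
; At zero HP it spawns blood, then after a delay destroys itself and spawns armor, bullet and HP pickups.
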(event Custom|CustomEvent
  (params (DeltaSeconds :type Float%20%28single-precision%29)))

(event EventBeginPlay
  (Audio|PlaySoundatLocation "/Game/CJW/Sounds/DogSound.DogSound" (Transformation|GetActorLocation) "0, 0, 0" 1.0 1.0 0.0 0 0 0 0))

(event Collision|EventActorBeginOverlap
  (params (OtherActor :type Actor%20Object%20Reference))
  ;[1 1 1] 적에게 닿으면 대미지를 주고 사라진다
  (Game|Damage|ApplyDamage OtherActor (Variables|Default|Getdamage) 0 0)
  (Actor|DestroyActor))

(event EventTick
  (params (DeltaSeconds :type Float%20%28single-precision%29))
  (bind _returnvalue (Transformation|GetActorLocation))
  (bind _returnvalue_2 (Transformation|GetActorLocation))
  (bind _returnvalue_3 (Utilities|Time|GetWorldDeltaSeconds))
  (bind _returnvalue_4 (Game|Player|GetPlayerPawn 0))
  (bind _speed (Variables|Default|GetSpeed))
  (bind _returnvalue_5 (Transformation|GetActorLocation _returnvalue_4))
  (bind _returnvalue_6 (- _returnvalue_5 _returnvalue_2))
  (bind _returnvalue_7 (Math|Vector|Normalize _returnvalue_6))
  (bind _returnvalue_8 (* _speed _returnvalue_7 _returnvalue_3))
  (bind _returnvalue_9 (+ _returnvalue _returnvalue_8))
  (Transformation|SetActorLocation (Math|Vector|MakeVector (.x _returnvalue_9) (.y _returnvalue_9) (.z _returnvalue_9)) false false)
  (Transformation|SetActorRotation (Math|Rotator|FindLookatRotation (Transformation|GetActorLocation (Game|Player|GetPlayerPawn 0)) (Transformation|GetActorLocation)))
  (Transformation|AddActorLocalRotation "0.000000,270.000000,0.000000" false false))

(event Game|Damage|EventAnyDamage
  (params (Damage :type Float%20%28single-precision%29) (DamageType :type Damage%20Type%20Object%20Reference) (InstigatedBy :type Controller%20Object%20Reference) (DamageCauser :type Actor%20Object%20Reference))
  (bind _returnvalue (Transformation|GetActorLocation))
  (bind _output_get (Variables|Default|SetHP (Math|Float|Truncate (- (Variables|Default|GetHP) Damage))))
  (Utilities|FlowControl|Sequence
    (:then_0
      (Transformation|SetActorLocation (+ (Transformation|GetActorLocation) (* (Math|Vector|Normalize (- (Transformation|GetActorLocation (Game|Player|GetPlayerPawn 0)) (Transformation|GetActorLocation))) "-15.000000,-15.000000,-15.000000")) false true))
    (:then_1
      (if (<= _output_get 0)
        (Effects|SpawnEmitteratLocation "/Game/Realistic_Starter_VFX_Pack_Vol2/Particles/Blood/P_Blood_Splat_Cone.P_Blood_Splat_Cone" (Transformation|GetActorLocation self) "0, 0, 0" "4.000000,4.000000,4.000000")
        (Utilities|FlowControl|Delay 0.5)
        (Actor|DestroyActor)
        (Utilities|FlowControl|Sequence
          (:then_0
            (Game|SpawnActorfromClass "/Game/CJW/BluePrints/BulletItem/Armor/BP_Armor.BP_Armor_C" (Math|Conversions|ToTransform(Vector) _returnvalue) "Undefined" "MultiplyWithRoot" 0 0))
          (:then_1
            (Game|SpawnActorfromClass "/Game/CJW/BluePrints/BulletItem/Bullet/BP_Bullet.BP_Bullet_C" (Math|Conversions|ToTransform(Vector) _returnvalue) "Undefined" "MultiplyWithRoot" 0 0))
          (:then_2
            (Game|SpawnActorfromClass "/Game/CJW/BluePrints/BulletItem/HP/BP_HP.BP_HP_C" (Math|Conversions|ToTransform(Vector) _returnvalue) "Undefined" "MultiplyWithRoot" 0 0)))
        (else
          (Utilities|FlowControl|Sequence
            (:then_0
              (if (<= (Variables|Default|GetHP) 50)
                (Variables|Default|SetIsGloryMode true)))))))))

(fn ConstructionScript)