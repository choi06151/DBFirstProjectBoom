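; Boss door Blueprint with two panels that slide apart to open and back together to close.
; Tick checks open and close flags, not set true in this file, and moves the panels by fixed per-frame offsets until that direction's step counter passes its limit, then clears the flag.
; Opening replays the door sound every frame, while closing is silent.
; Neither counter resets here.
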(event EventBeginPlay)

(event Collision|EventActorBeginOverlap
  (params (OtherActor :type Actor%20Object%20Reference)))

(event EventTick
  (params (DeltaSeconds :type Float%20%28single-precision%29))
  (Utilities|FlowControl|Sequence
    (:then_0
      (if (Variables|Default|GetIsDoorOpen)
        (if (<= (Variables|Default|GetDoorOpen) 1e+02)
          ;[1 1 1] 열린다
          (Utilities|FlowControl|Sequence
            (:then_0
              (Transformation|AddRelativeLocation (Variables|Default|GetDoorLeft) "-5.000000,0.000000,0.000000" false false)
              (Audio|PlaySound2D "/Game/CJW/Sounds/Door.Door" 1.0 1.0 0.0 0 0))
            (:then_1
              (Transformation|AddRelativeLocation (Variables|Default|GetDoorRight) "5.000000,0.000000,0.000000" false false)
              (Variables|Default|SetDoorOpen (+ (Variables|Default|GetDoorOpen) 1.0))
              (Audio|PlaySound2D "/Game/CJW/Sounds/Door.Door" 1.0 1.0 0.0 0 0)))
          (else
            (Variables|Default|SetIsDoorOpen false)))))
    (:then_1
      (if (Variables|Default|GetIsDoorClose)
        ;[1 1 1] 닫힌다
        (if (<= (Variables|Default|GetDoorClose) 1e+02)
          (Utilities|FlowControl|Sequence
            (:then_0
              (Transformation|AddRelativeLocation (Variables|Default|GetDoorLeft) "5.000000,0.000000,0.000000" false false))
            (:then_1
              (Transformation|AddRelativeLocation (Variables|Default|GetDoorRight) "-5.000000,0.000000,0.000000" false false)
              (Variables|Default|SetDoorClose (+ (Variables|Default|GetDoorClose) 1.0))))
          (else
            (Variables|Default|SetIsDoorClose false)))))))

(fn ConstructionScript)