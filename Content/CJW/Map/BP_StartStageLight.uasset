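; BP_StartStageLight is a stage-start indicator that switches its look once the player has triggered the start of a stage.
; Tick polls IsStageStart, which is not set in this Blueprint, and toggles visibility between the BeforeStart and AfterStart components.
; On the first tick with the flag true, it plays the 2D GameStart sound from an offset, using NewVar as a one-shot guard.
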(event EventBeginPlay)

(event Collision|EventActorBeginOverlap
  (params (OtherActor :type Actor%20Object%20Reference)))

(event EventTick
  (params (DeltaSeconds :type Float%20%28single-precision%29))
  (if (Variables|Default|GetIsStageStart)
    ;[1 1 1] 트리거를 밟은 후
    (Rendering|SetVisibility (Variables|Default|GetAfter%20Start) true false)
    (Rendering|SetVisibility (Variables|Default|GetBeforeStart) false false)
    (if (not (Variables|Default|GetNewVar))
      (Audio|PlaySound2D "/Game/CJW/Sounds/GameStart.GameStart" 1.0 1.0 39.0 0 0)
      (Variables|Default|SetNewVar true))
    (else
      ;[1 1 1] 트리거를 밟기 전
      (Rendering|SetVisibility (Variables|Default|GetBeforeStart) true false)
      (Rendering|SetVisibility (Variables|Default|GetAfter%20Start) false false))))

(fn ConstructionScript)