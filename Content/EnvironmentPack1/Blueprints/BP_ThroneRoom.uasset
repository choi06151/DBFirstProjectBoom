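; Throne room stage controller that stages a collapse intro, timed enemy waves and the opening of the exit.
; WhenStageStart spawns FS_MasterField actors with delayed collapse sounds, then enables Spawn.
; Tick counts frames to spawn four waves of fields and enemies at hard-coded locations.
; Stage clear follows a delay after the last wave, without checking kills, then destroys Angel and raises SMElevator and BrokenAngel per tick.
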(event Custom|WhenStageStart
  ;[1 1 1] 게임 시작전 대사출력
  (Utilities|FlowControl|Sequence
    (:then_1
      (Utilities|FlowControl|Sequence
        (:then_0
          (Game|SpawnActorfromClass "/Engine/EditorResources/FieldNodes/FS_MasterField.FS_MasterField_C" (Math|Transform|MakeTransform "-14070.000000,1080.000000,10430.000000" "0, 0, 0" "4.000000,4.000000,4.000000") "Undefined" "MultiplyWithRoot" 0 0)
          (Utilities|FlowControl|Delay 2.0)
          (Utilities|FlowControl|Sequence
            (:then_0
              (Game|SpawnActorfromClass "/Engine/EditorResources/FieldNodes/FS_MasterField.FS_MasterField_C" (Math|Transform|MakeTransform "-13380.000000,-2470.000000,10430.000000" "0, 0, 0" "4.000000,4.000000,4.000000") "Undefined" "MultiplyWithRoot" 0 0)
              (Utilities|FlowControl|Delay 3.0)
              (Utilities|FlowControl|Sequence
                (:then_0
                  (Game|SpawnActorfromClass "/Engine/EditorResources/FieldNodes/FS_MasterField.FS_MasterField_C" (Math|Transform|MakeTransform "-15040.000000,-720.000000,14010.000000" "0, 0, 0" "4.000000,4.000000,4.000000") "Undefined" "MultiplyWithRoot" 0 0)
                  (Utilities|FlowControl|Delay 4.0)
                  (Variables|Default|SetSpawn true))
                (:then_1
                  (Audio|PlaySound2D "/Game/JIU/StarterContent/Audio/Collapse02.Collapse02" 1.0 1.0 0.0 0 0))))
            (:then_1
              (Audio|PlaySound2D "/Game/JIU/StarterContent/Audio/Collapse01.Collapse01" 1.0 1.0 0.0 0 0))))
        (:then_1
          (Audio|PlaySound2D "/Game/JIU/StarterContent/Audio/Collapse01.Collapse01" 1.0 1.0 0.0 0 0))))))

(event EventBeginPlay)

(event Collision|EventActorBeginOverlap
  (params (OtherActor :type Actor%20Object%20Reference)))

(event EventTick
  (params (DeltaSeconds :type Float%20%28single-precision%29))
  (bind _angel (Variables|Default|GetAngel))
  (Utilities|FlowControl|Sequence
    (:then_0
      (if (Variables|Default|GetIsStageClear)
        ;[1 1 1] 1스테이지의 몹을 다 죽이면 , 물체가 파괴되서 아래로 내려갈수 있게 된다
        (if (<= (Variables|Default|GetHeight) 1e+02)
          (Transformation|AddRelativeLocation (Variables|Default|GetSM_Elevator) "0.000000,0.000000,10.000000" false false)
          (Variables|Default|SetHeight (+ (Variables|Default|GetHeight) 1.0))
          (Audio|PlaySound2D "/Game/CJW/Sounds/Door.Door" 1.0 1.0 0.0 0 0)
          (Utilities|IsValid _angel
            (:Is%20Valid
              (Components|DestroyComponent _angel))))))
    (:then_2
      (if (Variables|Default|GetSpawn)
        (Utilities|FlowControl|Sequence
          (:then_0
            (if (== (Variables|Default|GetTimeCycle) 6e+01)
              (Utilities|FlowControl|Sequence
                (:then_0
                  (Game|SpawnActorfromClass "/Engine/EditorResources/FieldNodes/FS_MasterField.FS_MasterField_C" (Math|Transform|MakeTransform "-18210.000000,-1440.000000,10400.000000" "0, 0, 0" "1.000000,1.000000,1.000000") "Undefined" "MultiplyWithRoot" 0 0)
                  (Game|SpawnActorfromClass "/Game/CJW/BluePrints/Enemy1_ShootGun/BP_Enemy1Boss/BP_Enemy1Boss.BP_Enemy1Boss_C" (Math|Transform|MakeTransform "-18210.000000,-1440.000000,10400.000000" "0, 0, 0" "1.000000,1.000000,1.000000") "Undefined" "MultiplyWithRoot" 0 0)
                  (Audio|PlaySound2D "/Game/CJW/Sounds/getdark.getdark" 1.0 1.0 0.0 0 0))
                (:then_1
                  (Game|SpawnActorfromClass "/Engine/EditorResources/FieldNodes/FS_MasterField.FS_MasterField_C" (Math|Transform|MakeTransform "-18149.000000,-79.999990,10400.000000" "0, 0, 0" "1.000000,1.000000,1.000000") "Undefined" "MultiplyWithRoot" 0 0)
                  (Game|SpawnActorfromClass "/Game/CJW/BluePrints/Enemy1_ShootGun/BP_Enemy1Boss/BP_Enemy1Boss.BP_Enemy1Boss_C" (Math|Transform|MakeTransform "-18149.000000,-79.999990,10400.000000" "0, 0, 0" "1.000000,1.000000,1.000000") "Undefined" "MultiplyWithRoot" 0 0))
                (:then_2
                  (Audio|PlaySound2D "/Game/JIU/StarterContent/Audio/Explosion01.Explosion01" 1.0 1.0 0.0 0 0))
                (:then_3
                  (Game|SpawnActorfromClass "/Game/CJW/BluePrints/Enemy2_Dogging/BP_Enemy2Hello.BP_Enemy2Hello_C" (Math|Transform|MakeTransform "-20380.000000,-2090.000000,10400.000000" "0, 0, 0" "1.000000,1.000000,1.000000") "Undefined" "MultiplyWithRoot" 0 0)
                  (Game|SpawnActorfromClass "/Game/CJW/BluePrints/Enemy2_Dogging/BP_Enemy2Hello.BP_Enemy2Hello_C" (Math|Transform|MakeTransform "-20380.000000,-800.000000,10400.000000" "0, 0, 0" "1.000000,1.000000,1.000000") "Undefined" "MultiplyWithRoot" 0 0)))))
          (:then_1
            (Variables|Default|SetTimeCycle (+ (Variables|Default|GetTimeCycle) 1.0)))
          (:then_2
            (if (== (Variables|Default|GetTimeCycle) 2e+02)
              (Utilities|FlowControl|Sequence
                (:then_0
                  (Game|SpawnActorfromClass "/Engine/EditorResources/FieldNodes/FS_MasterField.FS_MasterField_C" (Math|Transform|MakeTransform "-17350.000000,-1440.000000,10400.000000" "0, 0, 0" "1.000000,1.000000,1.000000") "Undefined" "MultiplyWithRoot" 0 0)
                  (Game|SpawnActorfromClass "/Game/CJW/BluePrints/Enemy1_ShootGun/BP_Enemy1Boss/BP_Enemy1Boss.BP_Enemy1Boss_C" (Math|Transform|MakeTransform "-17350.000000,-1440.000000,10400.000000" "0, 0, 0" "1.000000,1.000000,1.000000") "Undefined" "MultiplyWithRoot" 0 0))
                (:then_1
                  (Game|SpawnActorfromClass "/Engine/EditorResources/FieldNodes/FS_MasterField.FS_MasterField_C" (Math|Transform|MakeTransform "-17289.999999,-79.999990,10400.000000" "0, 0, 0" "1.000000,1.000000,1.000000") "Undefined" "MultiplyWithRoot" 0 0)
                  (Game|SpawnActorfromClass "/Game/CJW/BluePrints/Enemy1_ShootGun/BP_Enemy1Boss/BP_Enemy1Boss.BP_Enemy1Boss_C" (Math|Transform|MakeTransform "-17289.999999,79.999990,10400.000000" "0, 0, 0" "1.000000,1.000000,1.000000") "Undefined" "MultiplyWithRoot" 0 0))
                (:then_2
                  (Audio|PlaySound2D "/Game/JIU/StarterContent/Audio/Explosion01.Explosion01" 1.0 1.0 0.0 0 0)))))
          (:then_3
            (if (== (Variables|Default|GetTimeCycle) 4e+02)
              (Utilities|FlowControl|Sequence
                (:then_0
                  (Game|SpawnActorfromClass "/Engine/EditorResources/FieldNodes/FS_MasterField.FS_MasterField_C" (Math|Transform|MakeTransform "-16410.000000,-1440.000000,10400.000000" "0, 0, 0" "1.000000,1.000000,1.000000") "Undefined" "MultiplyWithRoot" 0 0)
                  (Game|SpawnActorfromClass "/Game/CJW/BluePrints/Enemy1_ShootGun/BP_Enemy1Boss/BP_Enemy1Boss.BP_Enemy1Boss_C" (Math|Transform|MakeTransform "-16410.000000,-1440.000000,10400.000000" "0, 0, 0" "1.000000,1.000000,1.000000") "Undefined" "MultiplyWithRoot" 0 0))
                (:then_1
                  (Game|SpawnActorfromClass "/Engine/EditorResources/FieldNodes/FS_MasterField.FS_MasterField_C" (Math|Transform|MakeTransform "-16349.999999,-79.999990,10400.000000" "0, 0, 0" "1.000000,1.000000,1.000000") "Undefined" "MultiplyWithRoot" 0 0)
                  (Game|SpawnActorfromClass "/Game/CJW/BluePrints/Enemy1_ShootGun/BP_Enemy1Boss/BP_Enemy1Boss.BP_Enemy1Boss_C" (Math|Transform|MakeTransform "-16349.999999,-79.999990,10400.000000" "0, 0, 0" "1.000000,1.000000,1.000000") "Undefined" "MultiplyWithRoot" 0 0))
                (:then_2
                  (Audio|PlaySound2D "/Game/JIU/StarterContent/Audio/Explosion01.Explosion01" 1.0 1.0 0.0 0 0))
                (:then_3
                  (Game|SpawnActorfromClass "/Game/CJW/BluePrints/Enemy2_Dogging/BP_Enemy2Hello.BP_Enemy2Hello_C" (Math|Transform|MakeTransform "-20380.000000,-2090.000000,10400.000000" "0, 0, 0" "1.000000,1.000000,1.000000") "Undefined" "MultiplyWithRoot" 0 0)
                  (Game|SpawnActorfromClass "/Game/CJW/BluePrints/Enemy2_Dogging/BP_Enemy2Hello.BP_Enemy2Hello_C" (Math|Transform|MakeTransform "-20380.000000,-800.000000,10400.000000" "0, 0, 0" "1.000000,1.000000,1.000000") "Undefined" "MultiplyWithRoot" 0 0)))))
          (:then_4
            (if (== (Variables|Default|GetTimeCycle) 6e+02)
              (Utilities|FlowControl|Sequence
                (:then_0
                  (Game|SpawnActorfromClass "/Engine/EditorResources/FieldNodes/FS_MasterField.FS_MasterField_C" (Math|Transform|MakeTransform "-15520.000000,-1440.000000,10400.000000" "0, 0, 0" "1.000000,1.000000,1.000000") "Undefined" "MultiplyWithRoot" 0 0)
                  (Game|SpawnActorfromClass "/Game/CJW/BluePrints/Enemy1_ShootGun/BP_Enemy1Boss/BP_Enemy1Boss.BP_Enemy1Boss_C" (Math|Transform|MakeTransform "-15520.000000,-1440.000000,10400.000000" "0, 0, 0" "1.000000,1.000000,1.000000") "Undefined" "MultiplyWithRoot" 0 0))
                (:then_1
                  (Game|SpawnActorfromClass "/Engine/EditorResources/FieldNodes/FS_MasterField.FS_MasterField_C" (Math|Transform|MakeTransform "-15459.999999,-79.999990,10400.000000" "0, 0, 0" "1.000000,1.000000,1.000000") "Undefined" "MultiplyWithRoot" 0 0)
                  (Game|SpawnActorfromClass "/Game/CJW/BluePrints/Enemy1_ShootGun/BP_Enemy1Boss/BP_Enemy1Boss.BP_Enemy1Boss_C" (Math|Transform|MakeTransform "-15459.999999,-79.999990,10400.000000" "0, 0, 0" "1.000000,1.000000,1.000000") "Undefined" "MultiplyWithRoot" 0 0))
                (:then_2
                  (Utilities|FlowControl|Delay 5.0)
                  (Variables|Default|SetIsStageClear true))
                (:then_3
                  (Audio|PlaySound2D "/Game/JIU/StarterContent/Audio/Explosion01.Explosion01" 1.0 1.0 0.0 0 0))))))))))

(fn ConstructionScript)